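; Ladder prefab that puts a BP_Character into climbing state while it overlaps the ladder's Box.
; Begin overlap sets Climbing, switches movement to Flying and opens a gate that lets Tick turn the character opposite the ladder's forward vector every frame.
; End overlap clears Climbing, switches movement to Falling and closes the gate.
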(event `self.ReceiveTick`
  (params (DeltaSeconds :type "Float (single-precision)"))
  (`/Engine/EditorBlueprintResources/StandardMacros.Gate` true :!label _label
    (:`Exit`
      (`self.K2_SetActorRotation` (stale `self.Box.OnComponentBeginOverlap` _asbp_character) (`KismetMathLibrary.Conv_VectorToRotator` (* (`self.GetActorForwardVector`) -1)) false))))

(event `self.Box.OnComponentBeginOverlap`
  (params (OverlappedComponent :type "PrimitiveComponent Object Reference") (OtherActor :type "Actor Object Reference") (OtherComp :type "PrimitiveComponent Object Reference") (OtherBodyIndex :type Integer) (bFromSweep :type Boolean) (SweepResult :type "HitResult Structure (by ref)"))
  (bind _asbp_character (cast `/Game/Blueprint/Character/BP_Character` OtherActor))
  (set `/Game/Blueprint/Character/BP_Character.Climbing` true _asbp_character)
  (`CharacterMovementComponent.SetMovementMode` (`Character.CharacterMovement` _asbp_character) "MOVE_Flying" 0)
  (goto _label :!via `Open`))

(event `self.Box.OnComponentEndOverlap`
  (params (OverlappedComponent :type "PrimitiveComponent Object Reference") (OtherActor :type "Actor Object Reference") (OtherComp :type "PrimitiveComponent Object Reference") (OtherBodyIndex :type Integer))
  (bind _asbp_character (cast `/Game/Blueprint/Character/BP_Character` OtherActor))
  (set `/Game/Blueprint/Character/BP_Character.Climbing` false _asbp_character)
  (`CharacterMovementComponent.SetMovementMode` (`Character.CharacterMovement` _asbp_character) "MOVE_Falling" 0)
  (goto _label :!via `Close`))

(fn `UserConstructionScript`)